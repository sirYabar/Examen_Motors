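; Coin-gated door that removes itself when the player has collected the required number of coins.
; A ThirdPersonCharacter entering the Box trigger makes it compare the game mode's coin count with NeededCoins.
; An exact match plays the Correct sound and destroys the actor; any other count plays Wrong.
; An OpenDoor function for sliding the mesh along world Y exists but is never called here.
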(event OnComponentBeginOverlap(Box)
  (params (OverlappedComponent :type Primitive%20Component%20Object%20Reference) (OtherActor :type Actor%20Object%20Reference) (OtherComp :type Primitive%20Component%20Object%20Reference) (OtherBodyIndex :type Integer) (bFromSweep :type Boolean) (SweepResult :type Hit%20Result%20Structure%20%28by%20ref%29))
  (bind _returnvalue (Transformation|GetActorLocation))
  (Utilities|Casting|CastToThirdPersonCharacter OtherActor)
  (bind _coins (Default|GetCoins (.AsThird%20Person%20Game%20Mode (Utilities|Casting|CastToThirdPersonGameMode (Game|GetGameMode)))))
  (if (== _coins (Variables|Default|GetNeededCoins))
    (Audio|PlaySoundatLocation "/Game/Sounds/correct.correct" _returnvalue "0, 0, 0" 1.0 1.0 0.0 0 0 0)
    (Actor|DestroyActor)
    (else
      (Audio|PlaySoundatLocation "/Game/Sounds/wrong.wrong" _returnvalue "0, 0, 0" 1.0 1.0 0.0 0 0 0))))

(event EventBeginPlay)

(event Collision|EventActorBeginOverlap
  (params (OtherActor :type Actor%20Object%20Reference)))

(event EventTick
  (params (DeltaSeconds :type Float%20%28single-precision%29)))

(fn ConstructionScript)

(fn OpenDoor
  (params (Deltatime :type Float%20%28single-precision%29))
  (bind _staticmesh (Variables|Default|GetStaticMesh))
  (bind _returnvalue (Transformation|GetWorldLocation _staticmesh))
  (if (not (< (.y _returnvalue) (Variables|Default|Getopened_y)))
    (Transformation|SetWorldLocation _staticmesh (Math|Vector|MakeVector (.x _returnvalue) (+ (* Deltatime 1e+03) (.y _returnvalue)) (.z _returnvalue)) false false)))